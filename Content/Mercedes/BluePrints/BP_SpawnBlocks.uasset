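; BP_SpawnBlocks is a one-shot trigger that spawns an actor when a BP_Character enters its Box.
; The overlap calls SpawnBlock, which spawns the ActorToSpawn class at the SpawnPoint component's world location.
; HasBeenUsed is set after that first call, so later overlaps only print an already-spawned debug message.
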(event `self.Box.OnComponentBeginOverlap`
  (params (OverlappedComponent :type "PrimitiveComponent Object Reference") (OtherActor :type "Actor Object Reference") (OtherComp :type "PrimitiveComponent Object Reference") (OtherBodyIndex :type Integer) (bFromSweep :type Boolean) (SweepResult :type "HitResult Structure (by ref)"))
  (cast `/Game/Dylan/Blueprints/BP_Character` OtherActor)
  (`self.SpawnBlock`)
  (set `self.HasBeenUsed` true))

(event `SpawnBlock`
  (if (`self.HasBeenUsed`)
    (`KismetSystemLibrary.PrintString` "Object has already Spawned")
    (else
      (`|SpawnActorFromClass` (`self.ActorToSpawn`) (`KismetMathLibrary.MakeTransform` (`SceneComponent.K2_GetComponentLocation` (`self.SpawnPoint`))) "Undefined" "MultiplyWithRoot" null null)
      (`KismetSystemLibrary.PrintString` "Object Spawn"))))

(fn `UserConstructionScript`)